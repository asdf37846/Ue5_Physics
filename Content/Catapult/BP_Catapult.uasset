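; Catapult Blueprint that is reloaded and then fired through successive presses of E.
; The first press runs a timeline that pitches the pull arm, then moves the projectile into place and marks the catapult loaded.
; A later press plays the launch timeline on the arm.
; When the arm overlaps a trigger box during launch, the projectile's rope constraint breaks and the cable end detaches, releasing the shot.
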(event `PressE`
  (bind _pullarm (`self.PullArm`))
  (if (`self.IsReload`)
    (set `self.Lanuch` true)
    (bind (_direction `_새_트랙_0`) (`Timeline|TL_Lanuch`)
      (:`Update`
        (`SceneComponent.K2_SetRelativeRotation` _pullarm (`KismetMathLibrary.MakeRotator` 0.0 `_새_트랙_0`) false false)))
    (elif (not (`self.IsClick`))
      (set `self.IsClick` true)
      (bind (_direction_2 `_새_트랙_0_2`) (`Timeline|TL_Reload`)
        (:`Update`
          (`SceneComponent.K2_SetRelativeRotation` _pullarm (`KismetMathLibrary.MakeRotator` 0.0 `_새_트랙_0_2`) false false))
        (:`Finished`
          (`KismetSystemLibrary.Delay` 0.2)
          (`KismetSystemLibrary.MoveComponentTo` (`self.Projectile`) (+ (`SceneComponent.RelativeLocation` (`self.Body`)) (0.0 5.0 110.0)) (struct :`Pitch` 10.0) false false 0.1)
          (set `self.IsReload` true))))))

(event `self.Box.OnComponentBeginOverlap`
  (params (OverlappedComponent :type "PrimitiveComponent Object Reference") (OtherActor :type "Actor Object Reference") (OtherComp :type "PrimitiveComponent Object Reference") (OtherBodyIndex :type Integer) (bFromSweep :type Boolean) (SweepResult :type "HitResult Structure (by ref)"))
  (if (== OtherComp (`self.Arm`))
    (if (`self.Lanuch`)
      (`PhysicsConstraintComponent.BreakConstraint` (`self.ProjectileRope`))
      (set `CableComponent.bAttachEnd` false (`self.Cable`)))))

(fn `UserConstructionScript`)